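; BP_BoxMask is an actor in the water post-process folder that tracks the player and toggles a mask parameter for materials.
; Every Tick it copies the player pawn's X, Y and yaw while keeping its own Z as a fixed reference height.
; It sets BOX_BP in the BOX_MASK parameter collection to 0 when the pawn is more than a small margin below that height, otherwise to 1.
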(event `self.ReceiveTick`
  (params (DeltaSeconds :type "Float (single-precision)"))
  (bind _returnvalue (`GameplayStatics.GetPlayerPawn` 0))
  (bind (_returnvalue_x _returnvalue_y _returnvalue_z) (`KismetMathLibrary.BreakVector` (`self.K2_GetActorLocation`)))
  (bind (_returnvalue_x_2 _returnvalue_y_2 _returnvalue_z_2) (`KismetMathLibrary.BreakVector` (`self.K2_GetActorLocation` _returnvalue)))
  (bind (_returnvalue_roll _returnvalue_pitch _returnvalue_yaw) (`KismetMathLibrary.BreakRotator` (`self.K2_GetActorRotation` _returnvalue)))
  (`self.K2_SetActorLocation` (`KismetMathLibrary.MakeVector` _returnvalue_x_2 _returnvalue_y_2 _returnvalue_z))
  (`self.K2_SetActorRotation` (`KismetMathLibrary.MakeRotator` 0.0 0.0 _returnvalue_yaw))
  (if (> (- _returnvalue_z _returnvalue_z_2) 5.0)
    (`KismetMaterialLibrary.SetScalarParameterValue` "/Game/Material/Water/WaterPostProcess/BOX_MASK.BOX_MASK" "BOX_BP")
    (else
      (`KismetMaterialLibrary.SetScalarParameterValue` "/Game/Material/Water/WaterPostProcess/BOX_MASK.BOX_MASK" "BOX_BP" 1.0))))

(fn `UserConstructionScript`)